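; Player character Blueprint with a camera-driven walk and look, crouch, flashlight toggle and interaction.
; Looping events add idle breathing sounds and camera shake, with further shakes on walking and crouching.
; A timeline lerps capsule height for crouching, while upward sphere traces block standing under obstacles, with gamepad rumble on a failed attempt.
; A per-tick camera sphere trace detects BPI_Interact actors, driving the HUD dot and opening the interact input's gate.
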(event Custom|PlayerCrouchCall
  (bind _returnvalue (Transformation|GetActorLocation))
  (bind _returnvalue_2 (Transformation|GetActorLocation))
  ;[0.05098 0.05098 0.05098] Input Crouch
  (Utilities|FlowControl|DoOnce false :!label _label
    (:Completed
      (if (Variables|CharacterMovement|GetBIsCrouch)
        (bind _returnvalue_3 (Collision|SphereTraceByChannel _returnvalue_2 (+ _returnvalue_2 (Math|Vector|MakeVector 0.0 0.0 104.0)) 16.0 "TraceTypeQuery1" false 0 "None"))
        (if (not _returnvalue_3)
          (Variables|CharacterMovement|SetBIsCrouch false)
          (Utilities|FlowControl|Sequence
            (:then_0
              ;;[0 0.0914 1] Camera Shake
              (Game|Feedback|ClientStartCameraShake (Game|GetPlayerController 0) "/Game/MyContents/MyBlueprints/Characters/Player/CameraShake/BP_CameraShakeCrouch.BP_CameraShakeCrouch_C" 1.0 "CameraLocal" "0, 0, 0" :!label _label_2))
            (:then_1
              (bind _crouchlerp (Timeline|CrouchTimeline ReverseFromEnd)
                (:Update
                  (Components|Capsule|SetCapsuleHalfHeight (Variables|Collision|GetCapsuleComponent) (Math|Float|Lerp 88.0 36.0 _crouchlerp) true)
                  (if (not (Variables|CharacterMovement|GetBIsCrouch))
                    (bind _returnvalue_4 (Collision|SphereTraceByChannel _returnvalue (+ _returnvalue (Math|Vector|MakeVector 0.0 0.0 104.0)) 16.0 "TraceTypeQuery1" false 0 "None"))
                    (if _returnvalue_4
                      (Variables|CharacterMovement|SetBIsCrouch true)
                      (Timeline|CrouchTimeline Reverse))))
                (:Finished
                  (Utilities|FlowControl|Sequence
                    (:then_0
                      (if (Variables|CharacterMovement|GetBIsCrouch)
                        (Character|Crouch)
                        (else
                          (Character|UnCrouch))))
                    (:then_1
                      (goto _label Reset)))))))
          (else
            (Variables|CharacterMovement|SetBIsCrouch true)
            ;;[0.1846 1 0] Controller Shake
            (CallFunction|AddControllerShake "/Game/MyContents/MyBlueprints/Characters/Player/ControllerShake/UnCrouchShakeFAIL.UnCrouchShakeFAIL")
            (goto _label Reset)))
        (else
          (Variables|CharacterMovement|SetBIsCrouch true)
          (Utilities|FlowControl|Sequence
            (:then_0
              (goto _label_2))
            (:then_1
              (Timeline|CrouchTimeline PlayFromStart))))))))

(event Custom|Idle%20Breathing%20Sound
  ;[1 0.7769 0] Idle Player Breathing Sound
  (Utilities|FlowControl|Delay (Variables|Default|GetBreathingIdleDeltaTimer))
  ;;[1 0.7769 0] Breath Idle Sound
  (Audio|PlaySoundatLocation "/Game/MyContents/MySounds/PlayerSound/BreathSound/Cue/Player_Breath_Inhale_Idle_Cue.Player_Breath_Inhale_Idle_Cue" (Transformation|GetWorldLocation (Variables|Default|GetCamera)) "0, 0, 0" 1.0 1.0 0.0 0 0 0 0)
  (Utilities|FlowControl|Delay 1.0)
  (Audio|PlaySoundatLocation "/Game/MyContents/MySounds/PlayerSound/BreathSound/Cue/Player_Breath_Exhale_Idle_Cue.Player_Breath_Exhale_Idle_Cue" (Transformation|GetWorldLocation (Variables|Default|GetCamera)) "0, 0, 0" 1.0 1.0 0.0 0 0 0 0)
  (Utilities|FlowControl|Delay 1.0)
  (Variables|Default|SetBreathingIdleDeltaTimer (Math|Random|RandomFloatinRange 5.0 15.0))
  (CallFunction|IdleBreathingSound))

(event Custom|IdlePlayerBreathing
  ;[0 0.0914 1] Idle Player Breathing Camera Effect
  ;;[0 0.0914 1] Camera Shake
  (Game|Feedback|ClientStartCameraShake (Game|GetPlayerController 0) "/Game/MyContents/MyBlueprints/Characters/Player/CameraShake/BP_CameraShakeIdle.BP_CameraShakeIdle_C" 1.0 "CameraLocal" "0, 0, 0")
  (Utilities|FlowControl|Delay 1.5)
  (CallFunction|IdlePlayerBreathing))

(event Input|EnhancedActionEvents|EnhancedInputActionIA_Walk
  (params (ActionValue :type Vector%202D%20Structure) (ElapsedSeconds :type Float%20%28double-precision%29) (TriggeredSeconds :type Float%20%28double-precision%29) (InputAction :type Input%20Action%20Object%20Reference :default "/Game/MyContents/MyBlueprints/Characters/Player/Inputs/IA_Walk.IA_Walk"))
  (bind _returnvalue (Game|GetPlayerController 0))
  ;[0.05098 0.05098 0.05098] Input Walk
  (if (not (Math|Float|InRange(Float) (.x ActionValue) -0.2 0.2))
    (Pawn|Input|AddMovementInput (Transformation|GetActorRightVector) (* (.x ActionValue) (Variables|CharacterMovement|GetWalkSpeedMultiplier)) false :!label _label)
    (Pawn|Input|AddMovementInput (Transformation|GetActorForwardVector) (* (.y ActionValue) (Variables|CharacterMovement|GetWalkSpeedMultiplier)) false)
    (if (not (Variables|CharacterMovement|GetBIsCrouch))
      ;;[0 0.0914 1] Camera Shake
      (Game|Feedback|ClientStartCameraShake _returnvalue "/Game/MyContents/MyBlueprints/Characters/Player/CameraShake/BP_CameraShakeWalk.BP_CameraShakeWalk_C" 1.0 "CameraLocal" "0, 0, 0")
      (else
        (Game|Feedback|ClientStartCameraShake _returnvalue "/Game/MyContents/MyBlueprints/Characters/Player/CameraShake/BP_CameraShakeWalk.BP_CameraShakeWalk_C" 0.65 "CameraLocal" "0, 0, 0")))
    (elif (not (Math|Float|InRange(Float) (.y ActionValue) -0.2 0.2))
      (goto _label))))

(event Input|EnhancedActionEvents|EnhancedInputActionIA_Interact
  (params (ActionValue :type Boolean) (ElapsedSeconds :type Float%20%28double-precision%29) (TriggeredSeconds :type Float%20%28double-precision%29) (InputAction :type Input%20Action%20Object%20Reference :default "/Game/MyContents/MyBlueprints/Characters/Player/Inputs/IA_Interact.IA_Interact"))
  ;[0.05098 0.05098 0.05098] Interact Raycast
  (:Completed
    (Utilities|FlowControl|Gate true
      (:Exit
        (Class|BPIInteract|Interaction(Message) (.hitactor (stale EventTick _outhit)) self (.hitcomponent (stale EventTick _outhit)))))))

(event Input|EnhancedActionEvents|EnhancedInputActionIA_Crouch
  (params (ActionValue :type Boolean) (ElapsedSeconds :type Float%20%28double-precision%29) (TriggeredSeconds :type Float%20%28double-precision%29) (InputAction :type Input%20Action%20Object%20Reference :default "/Game/MyContents/MyBlueprints/Characters/Player/Inputs/IA_Crouch.IA_Crouch"))
  (bind _returnvalue (Transformation|GetActorLocation))
  (bind _returnvalue_2 (Transformation|GetActorLocation))
  ;[0.05098 0.05098 0.05098] Input Crouch
  (:Started
    (Utilities|FlowControl|DoOnce false :!label _label
      (:Completed
        (if (Variables|CharacterMovement|GetBIsCrouch)
          (bind _returnvalue_3 (Collision|SphereTraceByChannel _returnvalue_2 (+ _returnvalue_2 (Math|Vector|MakeVector 0.0 0.0 104.0)) 16.0 "TraceTypeQuery1" false 0 "None"))
          (if (not _returnvalue_3)
            (Variables|CharacterMovement|SetBIsCrouch false)
            (Utilities|FlowControl|Sequence
              (:then_0
                ;;[0 0.0914 1] Camera Shake
                (Game|Feedback|ClientStartCameraShake (Game|GetPlayerController 0) "/Game/MyContents/MyBlueprints/Characters/Player/CameraShake/BP_CameraShakeCrouch.BP_CameraShakeCrouch_C" 1.0 "CameraLocal" "0, 0, 0" :!label _label_2))
              (:then_1
                (bind _crouchlerp (Timeline|CrouchTimeline ReverseFromEnd)
                  (:Update
                    (Components|Capsule|SetCapsuleHalfHeight (Variables|Collision|GetCapsuleComponent) (Math|Float|Lerp 88.0 36.0 _crouchlerp) true)
                    (if (not (Variables|CharacterMovement|GetBIsCrouch))
                      (bind _returnvalue_4 (Collision|SphereTraceByChannel _returnvalue (+ _returnvalue (Math|Vector|MakeVector 0.0 0.0 104.0)) 16.0 "TraceTypeQuery1" false 0 "None"))
                      (if _returnvalue_4
                        (Variables|CharacterMovement|SetBIsCrouch true)
                        (Timeline|CrouchTimeline Reverse))))
                  (:Finished
                    (Utilities|FlowControl|Sequence
                      (:then_0
                        (if (Variables|CharacterMovement|GetBIsCrouch)
                          (Character|Crouch)
                          (else
                            (Character|UnCrouch))))
                      (:then_1
                        (goto _label Reset)))))))
            (else
              (Variables|CharacterMovement|SetBIsCrouch true)
              ;;[0.1846 1 0] Controller Shake
              (CallFunction|AddControllerShake "/Game/MyContents/MyBlueprints/Characters/Player/ControllerShake/UnCrouchShakeFAIL.UnCrouchShakeFAIL")
              (goto _label Reset)))
          (else
            (Variables|CharacterMovement|SetBIsCrouch true)
            (Utilities|FlowControl|Sequence
              (:then_0
                (goto _label_2))
              (:then_1
                (Timeline|CrouchTimeline PlayFromStart)))))))))

(event Input|EnhancedActionEvents|EnhancedInputActionIA_ToggleLight
  (params (ActionValue :type Boolean) (ElapsedSeconds :type Float%20%28double-precision%29) (TriggeredSeconds :type Float%20%28double-precision%29) (InputAction :type Input%20Action%20Object%20Reference :default "/Game/MyContents/MyBlueprints/Characters/Player/Inputs/IA_ToggleLight.IA_ToggleLight"))
  ;[0.05098 0.05098 0.05098] Input Flashlight
  (:Started
    (bind _asbp_flashlight (Utilities|Casting|CastToBP_Flashlight (Variables|/Script/Engine.ChildActorComponent|GetChildActor (Variables|Default|GetBP_Flashlight))))
    (Default|ToggleFlashLight _asbp_flashlight)))

(event Input|EnhancedActionEvents|EnhancedInputActionIA_Look
  (params (ActionValue :type Vector%202D%20Structure) (ElapsedSeconds :type Float%20%28double-precision%29) (TriggeredSeconds :type Float%20%28double-precision%29) (InputAction :type Input%20Action%20Object%20Reference :default "/Game/MyContents/MyBlueprints/Characters/Player/Inputs/IA_Look.IA_Look"))
  ;[0.05098 0.05098 0.05098] Input Camera Look
  (Pawn|Input|AddControllerYawInput (* (.x ActionValue) (Variables|CharacterCamera|GetCameraRotateSpeedMultiplier)))
  (Pawn|Input|AddControllerPitchInput (* (.y ActionValue) (Variables|CharacterCamera|GetCameraRotateSpeedMultiplier))))

(event EventTick
  (params (DeltaSeconds :type Float%20%28single-precision%29))
  (bind _camera (Variables|Default|GetCamera))
  (bind _w_mainhud (Variables|Default|GetW_MainHUD))
  (bind _returnvalue (Transformation|GetWorldLocation _camera))
  ;[0.05098 0.05098 0.05098] Interact Raycast
  (Utilities|FlowControl|Sequence
    (:then_0
      (bind _outhit (Collision|SphereTraceByChannel _returnvalue (+ _returnvalue (* (Math|Vector|GetForwardVector _camera) (Variables|CharacterCamera|GetRaycastDistance))) 5.0 "TraceTypeQuery1" false 0 "None"))
      (if (Utilities|DoesObjectImplementInterface (.hitactor _outhit) "/Game/MyContents/MyBlueprints/Characters/Player/BPI_Interact.BPI_Interact_C")
        (Utilities|FlowControl|Sequence
          (:then_0
            (Utilities|FlowControl|Gate true) ; enters at Open
          )
          (:then_1
            (Utilities|FlowControl|DoOnce false :!label _label
              (:Completed
                (Default|ToggleInteractDot _w_mainhud)
                (goto _label_2 Reset)))))
        (else
          (Utilities|FlowControl|DoOnce false :!label _label_2
            (:Completed
              (Default|DisableInteractDot _w_mainhud)
              (goto _label Reset))))))))

(event EventBeginPlay
  ;[0.05098 0.05098 0.05098] Toggle Idle Breathing Camera Effect
  (CallFunction|IdlePlayerBreathing)
  ;[0.05098 0.05098 0.05098] Toggle Idle Breathing Sound
  (CallFunction|IdleBreathingSound)
  (bind _asmy_main_hud (Utilities|Casting|CastToMyMainHUD (HUD|GetHUD (Game|GetPlayerController 0))))
  (Variables|Default|SetW_MainHUD _asmy_main_hud))

(event Input|KeyboardEvents|DebugKeyU
  (params (Key :type Key%20Structure :default "None") (ActionValue :type Input%20Action%20Value%20Structure))
  (:Pressed
    (Default|ToggleInteractDot (Variables|Default|GetW_MainHUD))))

(fn ConstructionScript)

(fn AddControllerShake
  (params (ForceFeedBackEffect :type Force%20Feedback%20Effect%20Object%20Reference))
  (Game|Feedback|ClientPlayForceFeedback (Game|GetPlayerController 0) ForceFeedBackEffect "" false false false))