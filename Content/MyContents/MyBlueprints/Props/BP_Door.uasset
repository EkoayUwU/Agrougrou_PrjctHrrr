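; BP_Door is an interactive door that toggles open and closed, moving the player along with it.
; PlayerDoorSide compares camera forward to the door's right vector to choose front or back, ignoring other angles.
; Timelines slide the movement-locked player to that side's reference point, attach them, then swing door and handle before restoring walking; only the front path disables collision.
; A locked door instead shakes with a camera shake, gated by DoOnce.
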(event `/Game/MyContents/MyBlueprints/Characters/Player/BPI_Interact.Interaction`
  (params (PlayerRef :type "/Game/MyContents/MyBlueprints/Characters/Player/BP_Player Object Reference"))
  (set `self.Player Ref` PlayerRef)
  ;[0.05098 0.05098 0.05098] Door Locked
  (if (not (`self.BIsLocked`))
    ;[0.05098 0.05098 0.05098] Is Door Opening
    (if (not (`self.BIsOpening`))
      (set `self.BIsOpening` true)
      (bind _caseindex (`self.PlayerDoorSide`))
      (switch `int` _caseindex
        (:`0`
          (set `self.BIsOpening` false))
        (:`1`
          (`PrimitiveComponent.SetCollisionEnabled` (`self.Door_Frame_MSH`) "NoCollision")
          (`PrimitiveComponent.SetCollisionEnabled` (`self.Door_MSH`) "NoCollision")
          ;[0.05098 0.05098 0.05098] LockPlayerOnDoorFront
          (`CharacterMovementComponent.SetMovementMode` (`Character.CharacterMovement` (`self.Player Ref`)) "MOVE_None" 0)
          (bind (_direction _playermovementlerpvalue) (`Timeline|Timeline` :!via `PlayFromStart`)
            (:`Update`
              (bind _returnvalue_location (`KismetMathLibrary.BreakTransform` (`KismetMathLibrary.TLerp` (`KismetMathLibrary.MakeTransform` (`self.K2_GetActorLocation` (`self.Player Ref`))) (`KismetMathLibrary.MakeTransform` (`SceneComponent.K2_GetComponentLocation` (`self.FrontDoorPlayerRefPoint`))) _playermovementlerpvalue)))
              (`self.K2_SetActorLocation` (`self.Player Ref`) _returnvalue_location true false))
            (:`Finished`
              (`self.K2_AttachToComponent` (`self.Player Ref`) (`self.FrontDoorPlayerRefPoint`) "None" "KeepWorld" "KeepWorld" "KeepWorld" false)
              (if (not (`self.BIsOpen`)) :!label _label
                (set `self.BIsOpen` true)
                ;[0.05098 0.05098 0.05098] Door Movement
                (bind (_direction_2 _doorlerpvalue _handlelerpvalue) (`Timeline|DoorMovement` :!via `PlayFromStart` :!label _label_2)
                  (:`Update`
                    (`SceneComponent.K2_SetRelativeRotation` (`self.Door_Handle_MSH`) (`KismetMathLibrary.MakeRotator` 0.0 (`KismetMathLibrary.Lerp` 0.0 -35.0 _handlelerpvalue)) false false)
                    (`SceneComponent.K2_SetRelativeRotation` (`self.Door_MSH`) (`KismetMathLibrary.MakeRotator` 0.0 0.0 (`KismetMathLibrary.Lerp` 0.0 -90.0 _doorlerpvalue)) false false)
                    (`SceneComponent.K2_SetRelativeRotation` (`self.PointRef`) (`KismetMathLibrary.MakeRotator` 0.0 0.0 (`KismetMathLibrary.Lerp` 90.0 0.0 _doorlerpvalue)) false false))
                  (:`Finished`
                    (set `self.BIsOpening` false)
                    (`PrimitiveComponent.SetCollisionEnabled` (`self.Door_Frame_MSH`) "QueryAndPhysics")
                    (`PrimitiveComponent.SetCollisionEnabled` (`self.Door_MSH`) "QueryAndPhysics")
                    ;[0.05098 0.05098 0.05098] Unlock Player
                    (`CharacterMovementComponent.SetMovementMode` (`Character.CharacterMovement` (`self.Player Ref`)) "MOVE_Walking" 0)
                    (`self.K2_DetachFromActor` "KeepWorld" "KeepWorld" "KeepWorld")))
                (else
                  (set `self.BIsOpen` false)
                  (goto _label_2 :!via `ReverseFromEnd`))))))
        (:`2`
          ;[0.05098 0.05098 0.05098] LockPlayerOnDoorBack
          (`CharacterMovementComponent.SetMovementMode` (`Character.CharacterMovement` (`self.Player Ref`)) "MOVE_None" 0)
          (bind (_direction_3 _playermovementlerpvalue_2) (`Timeline|PlayerMovement` :!via `PlayFromStart`)
            (:`Update`
              (bind _returnvalue_location_2 (`KismetMathLibrary.BreakTransform` (`KismetMathLibrary.TLerp` (`KismetMathLibrary.MakeTransform` (`self.K2_GetActorLocation` (`self.Player Ref`))) (`KismetMathLibrary.MakeTransform` (`SceneComponent.K2_GetComponentLocation` (`self.BackDoorPlayerRefPoint`))) _playermovementlerpvalue_2)))
              (`self.K2_SetActorLocation` (`self.Player Ref`) _returnvalue_location_2 false false))
            (:`Finished`
              (`self.K2_AttachToComponent` (`self.Player Ref`) (`self.BackDoorPlayerRefPoint`) "None" "KeepWorld" "KeepWorld" "KeepWorld" false)
              (goto _label))))))
    (else
      ;[0.05098 0.05098 0.05098] Door Shake if Locked
      (`/Engine/EditorBlueprintResources/StandardMacros.DoOnce` false :!label _label_3
        (:`Completed`
          (`|ExecutionSequence`
            (:`then_0`
              (bind (_direction_4 _doorshakelerpvalue _handledoorshakelerpvalue) (`Timeline|DoorShake` :!via `PlayFromStart`)
                (:`Update`
                  (`SceneComponent.K2_SetRelativeRotation` (`self.Door_MSH`) (`KismetMathLibrary.MakeRotator` 0.0 0.0 (`KismetMathLibrary.Lerp` 0.0 -1.0 _doorshakelerpvalue)) false false)
                  (`SceneComponent.K2_SetRelativeRotation` (`self.Door_Handle_MSH`) (`KismetMathLibrary.MakeRotator` 0.0 (`KismetMathLibrary.Lerp` 0.0 -8.5 _handledoorshakelerpvalue)) false false)
                  (goto _label_3 :!via `Reset`))))
            (:`then_1`
              (`PlayerController.ClientStartCameraShake` :`self` (`PlayerState.GetPlayerController` (`Pawn.PlayerState` (`self.Player Ref`))) :`Shake` "/Game/MyContents/MyBlueprints/Characters/Player/CameraShake/BP_CameraShakeLockDoor.BP_CameraShakeLockDoor_C"))))))))

(fn `PlayerDoorSide`
  (returns (CaseIndex :type Integer))
  (bind _returnvalue (`KismetMathLibrary.Dot_VectorVector` (`SceneComponent.GetForwardVector` (`/Game/MyContents/MyBlueprints/Characters/Player/BP_Player.Camera` (`self.Player Ref`))) (`self.GetActorRightVector`)))
  (if (`KismetMathLibrary.NearlyEqual_FloatFloat` _returnvalue 1.0 0.65)
    (return 1)
    (elif (`KismetMathLibrary.NearlyEqual_FloatFloat` _returnvalue -1.0 0.65)
      (return 2)
      (else
        (return 0)))))

(fn `UserConstructionScript`)