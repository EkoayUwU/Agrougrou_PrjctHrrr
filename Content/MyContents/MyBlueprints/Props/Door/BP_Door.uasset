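; Interactive door that the player can open and close from either side, or lock pick when locked.
; A trigger box gates interaction, and the camera-to-door dot product picks front or back.
; Timelines glide the input-locked player to reference points, aim the camera, then swing the door and handle with sounds.
; Locked doors either shake with camera and controller feedback, or crouch the player at the handle and spawn BP_LockPicking.
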(event `self.ReceiveBeginPlay`
  ;[0.05098 0.05098 0.05098] Init Player Ref
  (bind _asbp_player (cast `/Game/MyContents/MyBlueprints/Characters/Player/BP_Player` (`GameplayStatics.GetPlayerPawn` 0)))
  (set `self.Player Ref` _asbp_player))

(event `/Game/MyContents/MyBlueprints/Characters/Player/BPI_Interact.Interaction`
  (params (PlayerRef :type "/Game/MyContents/MyBlueprints/Characters/Player/BP_Player Object Reference") (HittedComponent :type "PrimitiveComponent Object Reference"))
  (bind _player_ref (`self.Player Ref`))
  (bind (_returnvalue_x _returnvalue_y _returnvalue_z) (`KismetMathLibrary.BreakVector` (`SceneComponent.K2_GetComponentLocation` (`self.Door_Handle_MSH`))))
  (bind (_returnvalue_x_2 _returnvalue_y_2 _returnvalue_z_2) (`KismetMathLibrary.BreakVector` (`self.K2_GetActorLocation` (`self.Player Ref`))))
  (bind (_returnvalue_x_3 _returnvalue_y_3 _returnvalue_z_3) (`KismetMathLibrary.BreakVector` (`self.K2_GetActorLocation` (`self.Player Ref`))))
  (bind (_returnvalue_x_4 _returnvalue_y_4 _returnvalue_z_4) (`KismetMathLibrary.BreakVector` (`SceneComponent.K2_GetComponentLocation` (`self.Door_Handle_MSH`))))
  ;[0.05098 0.05098 0.05098] Interact By Player
  (if (== HittedComponent (`self.Door_MSH`))
    (set `self.Player Ref` PlayerRef)
    (`/Engine/EditorBlueprintResources/StandardMacros.Gate` true :!label _label
      (:`Exit`
        ;[0.05098 0.05098 0.05098] Door Locked
        (if (not (`self.BIsLocked`))
          ;[0.05098 0.05098 0.05098] Is Door Opening
          (if (not (`self.BIsOpening`))
            (set `self.BIsOpening` true)
            (bind _caseindex (`self.PlayerDoorSide`))
            (switch `int` _caseindex
              (:`0`
                (set `self.BIsOpening` false))
              (:`1`
                (`PrimitiveComponent.SetCollisionEnabled` (`self.Door_Frame_MSH`) "NoCollision")
                (`PrimitiveComponent.SetCollisionEnabled` (`self.Door_MSH`) "NoCollision")
                ;[0.05098 0.05098 0.05098] LockPlayerOnDoorFront
                (`CharacterMovementComponent.SetMovementMode` (`Character.CharacterMovement` (`self.Player Ref`)) "MOVE_None" 0)
                (bind (_direction _playermovementlerpvalue) (`Timeline|Timeline` :!via `PlayFromStart`)
                  (:`Update`
                    (bind _returnvalue_location (`KismetMathLibrary.BreakTransform` (`KismetMathLibrary.TLerp` (`KismetMathLibrary.MakeTransform` (`self.K2_GetActorLocation` (`self.Player Ref`))) (`KismetMathLibrary.MakeTransform` (`SceneComponent.K2_GetComponentLocation` (`self.FrontDoorPlayerRefPoint`))) _playermovementlerpvalue)))
                    (`self.K2_SetActorLocation` (`self.Player Ref`) _returnvalue_location true false))
                  (:`Finished`
                    (`self.K2_AttachToComponent` (`self.Player Ref`) (`self.FrontDoorPlayerRefPoint`) "None" "KeepWorld" "KeepWorld" "KeepWorld" false)
                    ;[0.05098 0.05098 0.05098] Set Camera Rotation
                    (`self.DisableInput` (`self.Player Ref`) (`GameplayStatics.GetPlayerController` 0) :!label _label_2)
                    (bind _targetedrotator (`self.WhereCamShouldAim`))
                    (`Timeline|Timeline_1` :!via `PlayFromStart`
                      (:`Update`
                        (`Controller.SetControlRotation` (`GameplayStatics.GetPlayerController` 0) (`KismetMathLibrary.RInterpTo` (`Pawn.GetControlRotation` (`self.Player Ref`)) _targetedrotator (`GameplayStatics.GetWorldDeltaSeconds`) 10.0)))
                      (:`Finished`
                        (if (not (`self.BIsOpen`))
                          (`|ExecutionSequence`
                            (:`then_0`
                              (set `self.BIsOpen` true)
                              ;[0.05098 0.05098 0.05098] Door Movement
                              (bind (_direction_2 _doorlerpvalue _handlelerpvalue) (`Timeline|DoorMovement` :!via `PlayFromStart` :!label _label_3)
                                (:`Update`
                                  (`SceneComponent.K2_SetRelativeRotation` (`self.Door_Handle_MSH`) (`KismetMathLibrary.MakeRotator` 0.0 (`KismetMathLibrary.Lerp` 0.0 -35.0 _handlelerpvalue)) false false)
                                  (`SceneComponent.K2_SetRelativeRotation` (`self.Door_MSH`) (`KismetMathLibrary.MakeRotator` 0.0 0.0 (`KismetMathLibrary.Lerp` 0.0 -90.0 _doorlerpvalue)) false false)
                                  (`SceneComponent.K2_SetRelativeRotation` (`self.PointRef`) (`KismetMathLibrary.MakeRotator` 0.0 0.0 (`KismetMathLibrary.Lerp` 90.0 0.0 _doorlerpvalue)) false false))
                                (:`Finished`
                                  (set `self.BIsOpening` false)
                                  (`PrimitiveComponent.SetCollisionEnabled` (`self.Door_Frame_MSH`) "QueryAndPhysics")
                                  (`PrimitiveComponent.SetCollisionEnabled` (`self.Door_MSH`) "QueryAndPhysics")
                                  ;[0.05098 0.05098 0.05098] Set Player To Crouch if was in this State
                                  (if (not (not (`/Game/MyContents/MyBlueprints/Characters/Player/BP_Player.BIsCrouch` (`self.Player Ref`))))
                                    (set `/Game/MyContents/MyBlueprints/Characters/Player/BP_Player.BIsCrouch` false _player_ref)
                                    (`/Game/MyContents/MyBlueprints/Characters/Player/BP_Player.PlayerCrouchCall` _player_ref))
                                  ;[0.05098 0.05098 0.05098] Unlock Player
                                  (`CharacterMovementComponent.SetMovementMode` (`Character.CharacterMovement` (`self.Player Ref`)) "MOVE_Walking" 0)
                                  (`self.K2_DetachFromActor` "KeepWorld" "KeepWorld" "KeepWorld")
                                  (`self.EnableInput` (`self.Player Ref`) (`GameplayStatics.GetPlayerController` 0)))))
                            (:`then_1`
                              ;[1 0.7769 0] Door Opening Sound
                              (`GameplayStatics.PlaySoundAtLocation` "/Game/MyContents/MySounds/PropsSound/DoorSound/Cue/Porte_Clence_Ouverture_Cue.Porte_Clence_Ouverture_Cue" (`KismetMathLibrary.MakeVector` _returnvalue_x _returnvalue_y _returnvalue_z) (struct) 1.0 1.0 0.0 null null null null)
                              (`GameplayStatics.PlaySoundAtLocation` "/Game/MyContents/MySounds/PropsSound/DoorSound/Sound/Porte_Ouverture_Sound.Porte_Ouverture_Sound" (+ (`SceneComponent.K2_GetComponentLocation` (`self.Door_MSH`)) (`KismetMathLibrary.MakeVector` 0.0 0.0 _returnvalue_z)) (struct) 1.0 1.0 0.0 null null null null)))
                          (else
                            (`|ExecutionSequence`
                              (:`then_0`
                                (set `self.BIsOpen` false)
                                (goto _label_3 :!via `ReverseFromEnd`))
                              (:`then_1`
                                ;[1 0.7769 0] Door Closing Sound
                                (`GameplayStatics.PlaySoundAtLocation` "/Game/MyContents/MySounds/PropsSound/DoorSound/Cue/Porte_Fermerture_Cue.Porte_Fermerture_Cue" (+ (`SceneComponent.K2_GetComponentLocation` (`self.Door_MSH`)) (`KismetMathLibrary.MakeVector` 0.0 0.0 _returnvalue_z_4)) (struct) 1.0 1.0 0.0 null null null null)
                                (`GameplayStatics.PlaySoundAtLocation` "/Game/MyContents/MySounds/PropsSound/DoorSound/Cue/Porte_Clence_Fermeture_Cue.Porte_Clence_Fermeture_Cue" (`KismetMathLibrary.MakeVector` _returnvalue_x_4 _returnvalue_y_4 _returnvalue_z_4) (struct) 1.0 1.0 0.0 null null null null))))))))))
              (:`2`
                ;[0.05098 0.05098 0.05098] LockPlayerOnDoorBack
                (`CharacterMovementComponent.SetMovementMode` (`Character.CharacterMovement` (`self.Player Ref`)) "MOVE_None" 0)
                (bind (_direction_3 _playermovementlerpvalue_2) (`Timeline|PlayerMovement` :!via `PlayFromStart`)
                  (:`Update`
                    (bind _returnvalue_location_2 (`KismetMathLibrary.BreakTransform` (`KismetMathLibrary.TLerp` (`KismetMathLibrary.MakeTransform` (`self.K2_GetActorLocation` (`self.Player Ref`))) (`KismetMathLibrary.MakeTransform` (`SceneComponent.K2_GetComponentLocation` (`self.BackDoorPlayerRefPoint`))) _playermovementlerpvalue_2)))
                    (`self.K2_SetActorLocation` (`self.Player Ref`) _returnvalue_location_2 false false))
                  (:`Finished`
                    (`self.K2_AttachToComponent` (`self.Player Ref`) (`self.BackDoorPlayerRefPoint`) "None" "KeepWorld" "KeepWorld" "KeepWorld" false)
                    (goto _label_2))))))
          (else
            ;[0.05098 0.05098 0.05098] Door Can Be Lock Pick ?
            (if (not (`self.BCanBeLockPick`))
              ;[0.05098 0.05098 0.05098] Door Shake if Locked
              (`/Engine/EditorBlueprintResources/StandardMacros.DoOnce` false :!label _label_4
                (:`Completed`
                  (`|ExecutionSequence`
                    (:`then_0`
                      (bind (_direction_4 _doorshakelerpvalue _handledoorshakelerpvalue) (`Timeline|DoorShake` :!via `PlayFromStart`)
                        (:`Update`
                          (`SceneComponent.K2_SetRelativeRotation` (`self.Door_MSH`) (`KismetMathLibrary.MakeRotator` 0.0 0.0 (`KismetMathLibrary.Lerp` 0.0 -1.0 _doorshakelerpvalue)) false false)
                          (`SceneComponent.K2_SetRelativeRotation` (`self.Door_Handle_MSH`) (`KismetMathLibrary.MakeRotator` 0.0 (`KismetMathLibrary.Lerp` 0.0 -8.5 _handledoorshakelerpvalue)) false false))
                        (:`Finished`
                          (goto _label_4 :!via `Reset`))))
                    (:`then_1`
                      ;;[0 0.0914 1] Camera Shake
                      (`PlayerController.ClientStartCameraShake` :`self` (`PlayerState.GetPlayerController` (`Pawn.PlayerState` (`self.Player Ref`))) :`Shake` "/Game/MyContents/MyBlueprints/Characters/Player/CameraShake/BP_CameraShakeLockDoor.BP_CameraShakeLockDoor_C")
                      ;;[0.1846 1 0] Controller Shake
                      (`/Game/MyContents/MyBlueprints/Characters/Player/BP_Player.Add Controller Shake` (`self.Player Ref`) "/Game/MyContents/MyBlueprints/Characters/Player/ControllerShake/Door/LockedDoorINTERACTION.LockedDoorINTERACTION")
                      ;;[1 0.7769 0] Lock Door Clapping Sound
                      (`GameplayStatics.PlaySoundAtLocation` "/Game/MyContents/MySounds/PropsSound/DoorSound/Cue/Door_Clap_Cue.Door_Clap_Cue" (`SceneComponent.K2_GetComponentLocation` (`self.Door_Handle_MSH`)) (struct) 1.0 1.0 0.0 null null null null)))))
              (else
                (`self.DisableInput` (`self.Player Ref`) (`GameplayStatics.GetPlayerController` 0))
                (bind _caseindex_2 (`self.PlayerDoorSide`))
                (switch `int` _caseindex_2
                  (:`1`
                    ;[0.05098 0.05098 0.05098] Set Player Position To Door Handle
                    (bind (_direction_5 _playermovementlerpvalue_3) (`Timeline|Timeline_3` :!via `PlayFromStart`)
                      (:`Update`
                        (bind _returnvalue (`KismetMathLibrary.TLerp` (`KismetMathLibrary.MakeTransform` (`KismetMathLibrary.MakeVector` _returnvalue_x_2 _returnvalue_y_2 _returnvalue_z_2)) (`KismetMathLibrary.MakeTransform` (`SceneComponent.K2_GetComponentLocation` (`self.FrontRefPointHandle`))) _playermovementlerpvalue_3))
                        (`self.K2_SetActorLocation` (`self.Player Ref`) (`KismetMathLibrary.MakeVector` (.x (.location _returnvalue)) (.y (.location _returnvalue)) _returnvalue_z_2) false false))
                      (:`Finished`
                        ;[0.05098 0.05098 0.05098] Set Player To Crouch if Not
                        (if (`/Game/MyContents/MyBlueprints/Characters/Player/BP_Player.BIsCrouch` (`self.Player Ref`)) :!label _label_5
                          ;[0.05098 0.05098 0.05098] Set Camera Rotation To Door Handle
                          (`Timeline|Timeline_2` :!via `PlayFromStart` :!label _label_6
                            (:`Update`
                              (`Controller.SetControlRotation` (`GameplayStatics.GetPlayerController` 0) (`KismetMathLibrary.RInterpTo` (`Pawn.GetControlRotation` (`self.Player Ref`)) (`KismetMathLibrary.FindLookAtRotation` (`SceneComponent.K2_GetComponentLocation` (`/Game/MyContents/MyBlueprints/Characters/Player/BP_Player.Camera` (`self.Player Ref`))) (`SceneComponent.K2_GetComponentLocation` (`self.Door_Handle_MSH`))) (`GameplayStatics.GetWorldDeltaSeconds`) 10.0)))
                            (:`Finished`
                              (`KismetSystemLibrary.Delay` 0.15)
                              ;[0.05098 0.05098 0.05098] Spawn LockPick MSH
                              (`|SpawnActorFromClass` "/Game/MyContents/MyBlueprints/Props/Door/BP_LockPicking.BP_LockPicking_C" (`KismetMathLibrary.MakeTransform` (0.0 0.0 -2000.0)) "Undefined" "MultiplyWithRoot" null (`self.Player Ref`) self null)))
                          (else
                            (`/Game/MyContents/MyBlueprints/Characters/Player/BP_Player.PlayerCrouchCall` (`self.Player Ref`))
                            (goto _label_6 :!via `PlayFromStart`))))))
                  (:`2`
                    ;[0.05098 0.05098 0.05098] Set Player Position To Door Handle
                    (bind (_direction_6 _playermovementlerpvalue_4) (`Timeline|Timeline_4` :!via `PlayFromStart`)
                      (:`Update`
                        (bind _returnvalue_2 (`KismetMathLibrary.TLerp` (`KismetMathLibrary.MakeTransform` (`KismetMathLibrary.MakeVector` _returnvalue_x_3 _returnvalue_y_3 _returnvalue_z_3)) (`KismetMathLibrary.MakeTransform` (`SceneComponent.K2_GetComponentLocation` (`self.BackRefPointHandle`))) _playermovementlerpvalue_4))
                        (`self.K2_SetActorLocation` (`self.Player Ref`) (`KismetMathLibrary.MakeVector` (.x (.location _returnvalue_2)) (.y (.location _returnvalue_2)) _returnvalue_z_3) false false))
                      (:`Finished`
                        (goto _label_5)))))))))))))

(event `self.Box.OnComponentBeginOverlap`
  (params (OverlappedComponent :type "PrimitiveComponent Object Reference") (OtherActor :type "Actor Object Reference") (OtherComp :type "PrimitiveComponent Object Reference") (OtherBodyIndex :type Integer) (bFromSweep :type Boolean) (SweepResult :type "HitResult Structure (by ref)"))
  ;[0.05098 0.05098 0.05098] Player In Range
  (if (== OtherActor (`self.Player Ref`))
    (goto _label :!via `Open`)))

(event `self.Box.OnComponentEndOverlap`
  (params (OverlappedComponent :type "PrimitiveComponent Object Reference") (OtherActor :type "Actor Object Reference") (OtherComp :type "PrimitiveComponent Object Reference") (OtherBodyIndex :type Integer))
  ;[0.05098 0.05098 0.05098] Player Not In Range
  (if (== OtherActor (`self.Player Ref`))
    (goto _label :!via `Close`)))

(fn `PlayerDoorSide`
  (returns (CaseIndex :type Integer))
  (bind _returnvalue (`KismetMathLibrary.Dot_VectorVector` (`SceneComponent.GetForwardVector` (`/Game/MyContents/MyBlueprints/Characters/Player/BP_Player.Camera` (`self.Player Ref`))) (`self.GetActorRightVector`)))
  (if (`KismetMathLibrary.NearlyEqual_FloatFloat` _returnvalue 1.0 0.8)
    (return 1)
    (elif (`KismetMathLibrary.NearlyEqual_FloatFloat` _returnvalue -1.0 0.85)
      (return 2)
      (else
        (return 0)))))

(fn `UserConstructionScript`)

(fn `WhereCamShouldAim`
  (returns (TargetedRotator :type "Rotator Structure"))
  (locals (TargetedPoint :type "StaticMeshComponent Object Reference"))
  (bind _caseindex (`self.PlayerDoorSide`))
  (switch `int` _caseindex
    (:`1`
      (if (`self.BIsOpen`)
        (set `local.TargetedPoint` (`self.CameraPointRef1Opened`))
        (else
          (set `local.TargetedPoint` (`self.CameraPointRef1Closed`)))))
    (:`2`
      (if (`self.BIsOpen`)
        (set `local.TargetedPoint` (`self.CameraPointRef2Opened`))
        (else
          (set `local.TargetedPoint` (`self.CameraPointRef2Closed`))))))
  (return (`KismetMathLibrary.FindLookAtRotation` (`SceneComponent.K2_GetComponentLocation` (`/Game/MyContents/MyBlueprints/Characters/Player/BP_Player.Camera` (`self.Player Ref`))) (`SceneComponent.K2_GetComponentLocation` (`local.TargetedPoint`)))))