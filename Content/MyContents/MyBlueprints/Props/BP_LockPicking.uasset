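; Lock-picking minigame actor that takes over player input and displays itself through a widget and isolated scene capture, wearing the owner door's material.
; Input rotates the pin while Tick compares its angle to a random target using nested, wrap-aware far, near and exact tolerances, layering controller shakes as haptic hints.
; Holding the exact angle runs a looping timer that unlocks LockOwner; unlocking or leaving restores player input and destroys the actor.
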(event `self.ReceiveBeginPlay`
  ;[0.05098 0.05098 0.05098] Begin
  (`self.Init Camera`)
  (`self.Init Lock Picking Interface`)
  (`self.SetLockMaterial`)
  ;[1 0 0] Connect When Everything is Done
  (`self.GenerateRandomRightValue`)
  (`KismetSystemLibrary.PrintString` (`KismetStringLibrary.Concat_StrStr` "Find " (`KismetStringLibrary.Conv_DoubleToString` (`self.RightRotValue`)))))

(event `Init Camera`
  ;[0.05098 0.05098 0.05098] Camera Init
  (`ComposureBlueprintLibrary.CopyCameraSettingsToSceneCapture` (`/Game/MyContents/MyBlueprints/Characters/Player/BP_Player.Camera` (`self.Player_Ref`)) (`self.SceneCaptureComponent2D`) 1.0)
  (`SceneComponent.ResetRelativeTransform` (`self.SceneCaptureComponent2D`)))

(event `Init Lock Picking Interface`
  ;[0.05098 0.05098 0.05098] LockPick Widget Interface Init
  (bind _returnvalue (`|CreateWidget` "/Game/MyContents/MyBlueprints/Widgets/WBP_LockPicking.WBP_LockPicking_C"))
  (bind _output_get (set `self.W_LPInterface` _returnvalue))
  (`UserWidget.AddToViewport` _output_get 0)
  (`Widget.SetVisibility` (`self.W_LPInterface`) "Visible")
  (`SceneCaptureComponent.ShowOnlyActorComponents` (`self.SceneCaptureComponent2D`) self false)
  (`self.DisableInput` (`self.Player_Ref`) (`GameplayStatics.GetPlayerController` 0))
  (`self.EnableInput` (`GameplayStatics.GetPlayerController` 0)))

(event `self.ReceiveTick`
  (params (DeltaSeconds :type "Float (single-precision)"))
  ;[0.05098 0.05098 0.05098] Lock System
  (`|ExecutionSequence`
    (:`then_0`
      ;;[0.05098 0.05098 0.05098] Check Lock Value
      (`self.RotationValueChecker`))
    (:`then_1`
      (if (`self.BIsOnRightValue`)
        (`/Engine/EditorBlueprintResources/StandardMacros.DoOnce` false :!label _label
          (:`Completed`
            ;;[0.05098 0.05098 0.05098] Time Handler On Right Value
            (bind _returnvalue (`KismetSystemLibrary.K2_SetTimer` null "TimerHandler" 0.35 true))))
        (else
          (`KismetSystemLibrary.K2_ClearAndInvalidateTimerHandle` _returnvalue)
          (set `self.TimerValue` 0)
          (goto _label :!via `Reset`))))))

(event `EnhancedInput|/Game/MyContents/MyBlueprints/Characters/Player/Inputs/IA_LockPicking`
  (params (ActionValue :type "Float (double-precision)") (ElapsedSeconds :type "Float (double-precision)") (TriggeredSeconds :type "Float (double-precision)") (InputAction :type "InputAction Object Reference" :default "/Game/MyContents/MyBlueprints/Characters/Player/Inputs/IA_LockPicking.IA_LockPicking"))
  ;[0.05098 0.05098 0.05098] Input Pin Rotation
  (:`Triggered`
    (bind _output_get (set `self.CurrentRotValue` (+ (* ActionValue 1.35) (`self.CurrentRotValue`))))
    (if (> (`self.CurrentRotValue`) 0.0)
      (if (< (`self.CurrentRotValue`) 360.0)
        (`SceneComponent.K2_SetRelativeRotation` (`self.PinRotationPivot`) (`KismetMathLibrary.MakeRotator` 0.0 _output_get) false false)
        (else
          (bind _output_get_2 (set `self.CurrentRotValue` 0.0))
          (`SceneComponent.K2_SetRelativeRotation` (`self.PinRotationPivot`) (`KismetMathLibrary.MakeRotator` 0.0 _output_get_2) false false)))
      (else
        (bind _output_get_3 (set `self.CurrentRotValue` 360.0))
        (`SceneComponent.K2_SetRelativeRotation` (`self.PinRotationPivot`) (`KismetMathLibrary.MakeRotator` 0.0 _output_get_3) false false)))))

(event `EnhancedInput|/Game/MyContents/MyBlueprints/Characters/Player/Inputs/IA_Leave`
  (params (ActionValue :type Boolean) (ElapsedSeconds :type "Float (double-precision)") (TriggeredSeconds :type "Float (double-precision)") (InputAction :type "InputAction Object Reference" :default "/Game/MyContents/MyBlueprints/Characters/Player/Inputs/IA_Leave.IA_Leave"))
  ;[0.05098 0.05098 0.05098] Leave LP Interface
  (:`Started`
    (`self.LeaveLPInterface`)))

(fn `GenerateRandomRightValue`
  (set `self.RightRotValue` (`KismetMathLibrary.RandomFloatInRange` 0.0 360.0)))

(fn `LeaveLPInterface`
  (`self.EnableInput` (`self.Player_Ref`) (`GameplayStatics.GetPlayerController` 0))
  (`Widget.RemoveFromParent` (`self.W_LPInterface`))
  (`self.K2_DestroyActor` self))

(fn `RotationValueChecker`
  ;[0.05098 0.05098 0.05098] FAR Right Rot
  (if (< (+ (`self.RightRotValue`) (`self.FarTolerance`)) 360.0)
    (if (> (- (`self.RightRotValue`) (`self.FarTolerance`)) 0.0)
      (if (`KismetMathLibrary.NearlyEqual_FloatFloat` (`self.CurrentRotValue`) (`self.RightRotValue`) (`self.FarTolerance`))
        ;[0.1846 1 0] Controller Shake
        (`/Game/MyContents/MyBlueprints/Characters/Player/BP_Player.Add Controller Shake` (`self.Player_Ref`) "/Game/MyContents/MyBlueprints/Characters/Player/ControllerShake/Door/LockPickingShakeFAR.LockPickingShakeFAR" :!label _label)
        ;[0.05098 0.05098 0.05098] NEAR Right Rot
        (if (< (+ (`self.RightRotValue`) (`self.NearTolerance`)) 360.0)
          (if (> (- (`self.RightRotValue`) (`self.NearTolerance`)) 0.0)
            (if (`KismetMathLibrary.NearlyEqual_FloatFloat` (`self.CurrentRotValue`) (`self.RightRotValue`) (`self.NearTolerance`))
              ;[0.1846 1 0] Controller Shake
              (`/Game/MyContents/MyBlueprints/Characters/Player/BP_Player.Add Controller Shake` (`self.Player_Ref`) "/Game/MyContents/MyBlueprints/Characters/Player/ControllerShake/Door/LockPickingShakeNEAR.LockPickingShakeNEAR" :!label _label_2)
              ;[0.05098 0.05098 0.05098] ON Right Rot
              (if (< (+ (`self.RightRotValue`) (`self.OnTolerance`)) 360.0)
                (if (> (- (`self.RightRotValue`) (`self.OnTolerance`)) 0.0)
                  (if (`KismetMathLibrary.NearlyEqual_FloatFloat` (`self.CurrentRotValue`) (`self.RightRotValue`) (`self.OnTolerance`))
                    ;[0.1846 1 0] Controller Shake
                    (`/Game/MyContents/MyBlueprints/Characters/Player/BP_Player.Add Controller Shake` (`self.Player_Ref`) "/Game/MyContents/MyBlueprints/Characters/Player/ControllerShake/Door/LockPickingShakeON.LockPickingShakeON" :!label _label_3)
                    (set `self.BIsOnRightValue` true)
                    (else
                      (set `self.BIsOnRightValue` false)))
                  (elif (or (`KismetMathLibrary.NearlyEqual_FloatFloat` (`self.CurrentRotValue`) (`self.RightRotValue`) (`self.OnTolerance`)) (`KismetMathLibrary.NearlyEqual_FloatFloat` (`self.CurrentRotValue`) 360.0 (`KismetMathLibrary.Abs` (- (`self.RightRotValue`) (`self.OnTolerance`)))))
                    (goto _label_3)
                    (else
                      (set `self.BIsOnRightValue` false))))
                (elif (or (`KismetMathLibrary.NearlyEqual_FloatFloat` (`self.CurrentRotValue`) (`self.RightRotValue`) (`self.OnTolerance`)) (`KismetMathLibrary.NearlyEqual_FloatFloat` (`self.CurrentRotValue`) 0.0 (- (+ (`self.RightRotValue`) (`self.OnTolerance`)) 360.0)))
                  (goto _label_3)
                  (else
                    (set `self.BIsOnRightValue` false))))
              (else
                (set `self.BIsOnRightValue` false)))
            (elif (or (`KismetMathLibrary.NearlyEqual_FloatFloat` (`self.CurrentRotValue`) (`self.RightRotValue`) (`self.NearTolerance`)) (`KismetMathLibrary.NearlyEqual_FloatFloat` (`self.CurrentRotValue`) 360.0 (`KismetMathLibrary.Abs` (- (`self.RightRotValue`) (`self.NearTolerance`)))))
              (goto _label_2)
              (else
                (set `self.BIsOnRightValue` false))))
          (elif (or (`KismetMathLibrary.NearlyEqual_FloatFloat` (`self.CurrentRotValue`) (`self.RightRotValue`) (`self.NearTolerance`)) (`KismetMathLibrary.NearlyEqual_FloatFloat` (`self.CurrentRotValue`) 0.0 (- (+ (`self.RightRotValue`) (`self.NearTolerance`)) 360.0)))
            (goto _label_2)
            (else
              (set `self.BIsOnRightValue` false))))
        (else
          (set `self.BIsOnRightValue` false)))
      (elif (or (`KismetMathLibrary.NearlyEqual_FloatFloat` (`self.CurrentRotValue`) (`self.RightRotValue`) (`self.FarTolerance`)) (`KismetMathLibrary.NearlyEqual_FloatFloat` (`self.CurrentRotValue`) 360.0 (`KismetMathLibrary.Abs` (- (`self.RightRotValue`) (`self.FarTolerance`)))))
        (goto _label)
        (else
          (set `self.BIsOnRightValue` false))))
    (elif (or (`KismetMathLibrary.NearlyEqual_FloatFloat` (`self.CurrentRotValue`) (`self.RightRotValue`) (`self.FarTolerance`)) (`KismetMathLibrary.NearlyEqual_FloatFloat` (`self.CurrentRotValue`) 0.0 (- (+ (`self.RightRotValue`) (`self.FarTolerance`)) 360.0)))
      (goto _label)
      (else
        (set `self.BIsOnRightValue` false)))))

(fn `SetLockMaterial`
  (`PrimitiveComponent.SetMaterial` (`self.Lock_MSH`) 0 (`PrimitiveComponent.GetMaterial` (`/Game/MyContents/MyBlueprints/Props/BP_Door.Door_MSH` (`self.LockOwner`)) 0)))

(fn `TimerHandler`
  (if (< (`self.TimerValue`) 4.0)
    (`/Engine/EditorBlueprintResources/StandardMacros.IncrementInt` (`self.TimerValue`))
    (else
      (set `/Game/MyContents/MyBlueprints/Props/BP_Door.BCanBeLockPick` false (`self.LockOwner`))
      (set `/Game/MyContents/MyBlueprints/Props/BP_Door.BIsLocked` false (`self.LockOwner`))
      ;[0.1846 1 0] Controller Shake
      (`/Game/MyContents/MyBlueprints/Characters/Player/BP_Player.Add Controller Shake` (`self.Player_Ref`) "/Game/MyContents/MyBlueprints/Characters/Player/ControllerShake/Door/LockPickingShakeONDuration.LockPickingShakeONDuration")
      ;[1 0.7769 0] Add Sound
      (`KismetSystemLibrary.PrintString` "UNLOCK")
      (`self.LeaveLPInterface`))))

(fn `UserConstructionScript`)