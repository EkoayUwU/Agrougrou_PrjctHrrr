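; BP_LockPicking is a work-in-progress lockpicking minigame actor that takes over player input and shows a pin through a scene capture and UMG widget.
; Input rotates the pin with 0–360 wraparound, while Tick compares its angle to a target using nested tolerance bands.
; A hit triggers TimerHandler once, but that function is empty and random target generation is unconnected.
; Leaving restores player input, removes the widget and destroys the actor.
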(event `self.ReceiveBeginPlay`
  ;[0.05098 0.05098 0.05098] Begin
  (`self.Init Camera`)
  (`self.Init Lock Picking Interface`))

(event `Init Camera`
  ;[0.05098 0.05098 0.05098] Camera Init
  (`ComposureBlueprintLibrary.CopyCameraSettingsToSceneCapture` (`/Game/MyContents/MyBlueprints/Characters/Player/BP_Player.Camera` (`self.Player_Ref`)) (`self.SceneCaptureComponent2D`) 1.0)
  (`SceneComponent.ResetRelativeTransform` (`self.SceneCaptureComponent2D`)))

(event `Init Lock Picking Interface`
  ;[0.05098 0.05098 0.05098] LockPick Widget Interface Init
  (bind _returnvalue (`|CreateWidget` "/Game/MyContents/MyBlueprints/Widgets/WBP_LockPicking.WBP_LockPicking_C"))
  (bind _output_get (set `self.W_LPInterface` _returnvalue))
  (`UserWidget.AddToViewport` _output_get 0)
  (`Widget.SetVisibility` (`self.W_LPInterface`) "Visible")
  (`SceneCaptureComponent.ShowOnlyActorComponents` (`self.SceneCaptureComponent2D`) self false)
  (`self.DisableInput` (`self.Player_Ref`) (`GameplayStatics.GetPlayerController` 0))
  (`self.EnableInput` (`GameplayStatics.GetPlayerController` 0)))

(event `self.ReceiveTick`
  (params (DeltaSeconds :type "Float (single-precision)"))
  ;[0.05098 0.05098 0.05098] Lock System
  (`|ExecutionSequence`
    (:`then_0`
      ;;[0.05098 0.05098 0.05098] Check Lock Value
      (`self.RotationValueChecker`))
    (:`then_1`
      (if (`self.BIsOnRightValue`)
        (`/Engine/EditorBlueprintResources/StandardMacros.DoOnce` false :!label _label
          (:`Completed`
            ;;[0.05098 0.05098 0.05098] Time Handler On Right Value
            (`self.TimerHandler`)))
        (else
          (goto _label :!via `Reset`))))))

(event `EnhancedInput|/Game/MyContents/MyBlueprints/Characters/Player/Inputs/IA_LockPicking`
  (params (ActionValue :type "Float (double-precision)") (ElapsedSeconds :type "Float (double-precision)") (TriggeredSeconds :type "Float (double-precision)") (InputAction :type "InputAction Object Reference" :default "/Game/MyContents/MyBlueprints/Characters/Player/Inputs/IA_LockPicking.IA_LockPicking"))
  ;[0.05098 0.05098 0.05098] Input Pin Rotation
  (:`Triggered`
    (bind _output_get (set `self.CurrentRotValue` (+ (* ActionValue 1.35) (`self.CurrentRotValue`))))
    (if (> (`self.CurrentRotValue`) 0.0)
      (if (< (`self.CurrentRotValue`) 360.0)
        (`SceneComponent.K2_SetRelativeRotation` (`self.PinRotationPivot`) (`KismetMathLibrary.MakeRotator` 0.0 _output_get) false false)
        (else
          (bind _output_get_2 (set `self.CurrentRotValue` 0.0))
          (bind _returnvalue (`KismetMathLibrary.MakeRotator` 0.0 _output_get_2))
          (`SceneComponent.K2_SetRelativeRotation` (`self.PinRotationPivot`) _returnvalue false false)
          (`KismetSystemLibrary.PrintString` (`KismetStringLibrary.Concat_StrStr` "GGGGGGGGGGGGG" (`KismetStringLibrary.Conv_RotatorToString` _returnvalue)))))
      (else
        (bind _output_get_3 (set `self.CurrentRotValue` 360.0))
        (bind _returnvalue_2 (`KismetMathLibrary.MakeRotator` 0.0 _output_get_3))
        (`SceneComponent.K2_SetRelativeRotation` (`self.PinRotationPivot`) _returnvalue_2 false false)
        (`KismetSystemLibrary.PrintString` (`KismetStringLibrary.Concat_StrStr` "GGGGGGGGGGGGG" (`KismetStringLibrary.Conv_RotatorToString` _returnvalue_2)))))))

(event `EnhancedInput|/Game/MyContents/MyBlueprints/Characters/Player/Inputs/IA_Leave`
  (params (ActionValue :type Boolean) (ElapsedSeconds :type "Float (double-precision)") (TriggeredSeconds :type "Float (double-precision)") (InputAction :type "InputAction Object Reference" :default "/Game/MyContents/MyBlueprints/Characters/Player/Inputs/IA_Leave.IA_Leave"))
  ;[0.05098 0.05098 0.05098] Leave LP Interface
  (:`Started`
    (`self.LeaveLPInterface`)))

(fn `GenerateRandomRightValue`
  (set `self.RightRotValue` (`KismetMathLibrary.RandomFloatInRange` 0.0 360.0)))

(fn `LeaveLPInterface`
  (`self.EnableInput` (`self.Player_Ref`) (`GameplayStatics.GetPlayerController` 0))
  (`Widget.RemoveFromParent` (`self.W_LPInterface`))
  (`self.K2_DestroyActor` self))

(fn `RotationValueChecker`
  (bind _currentrotvalue (`self.CurrentRotValue`))
  (bind _rightrotvalue (`self.RightRotValue`))
  (bind _currentrotvalue_2 (`self.CurrentRotValue`))
  (bind _rightrotvalue_2 (`self.RightRotValue`))
  (bind _currentrotvalue_3 (`self.CurrentRotValue`))
  (bind _rightrotvalue_3 (`self.RightRotValue`))
  (if (and (>= _currentrotvalue_2 (+ _rightrotvalue_2 -15.0)) (<= _currentrotvalue_2 (+ _rightrotvalue_2 15.0)))
    (if (and (>= _currentrotvalue_3 (+ _rightrotvalue_3 -6.25)) (<= _currentrotvalue_3 (+ _rightrotvalue_3 6.25)))
      (if (and (>= _currentrotvalue (+ _rightrotvalue -1.25)) (<= _currentrotvalue (+ _rightrotvalue 1.25)))
        (`KismetSystemLibrary.PrintString` "WP")
        (set `self.BIsOnRightValue` true)
        (else
          (`KismetSystemLibrary.PrintString` (`KismetStringLibrary.Concat_StrStr` "Close To " (`KismetStringLibrary.Conv_DoubleToString` (`self.RightRotValue`))))
          (set `self.BIsOnRightValue` false)))
      (else
        (set `self.BIsOnRightValue` false)))
    (else
      (set `self.BIsOnRightValue` false))))

(fn `TimerHandler`)

(fn `UserConstructionScript`)