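; Interactable note prop that lets the player read its text in a full-screen HUD widget.
; Interaction hides the paper mesh, plays a paper sound, shows WBP_NotesHUD with the note text, and moves input from the player to the note.
; The IA_Leave action reverses this, removing the widget and restoring the mesh and player input.
; A ReloadTexture event applies a random sheet material from the DT_Notes_MAT data table.
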(event `/Game/MyContents/MyBlueprints/Characters/Player/BPI_Interact.Interaction`
  (params (PlayerRef :type "/Game/MyContents/MyBlueprints/Characters/Player/BP_Player Object Reference") (HittedComponent :type "PrimitiveComponent Object Reference"))
  ;[0.05098 0.05098 0.05098] Open Note HUD
  (set `self.Player Ref` PlayerRef)
  (if (not (`self.BIsPlayerReading`))
    (`self.ToggleReading`)))

(event `EnhancedInput|/Game/MyContents/MyBlueprints/Characters/Player/Inputs/IA_Leave`
  (params (ActionValue :type Boolean) (ElapsedSeconds :type "Float (double-precision)") (TriggeredSeconds :type "Float (double-precision)") (InputAction :type "InputAction Object Reference" :default "/Game/MyContents/MyBlueprints/Characters/Player/Inputs/IA_Leave.IA_Leave"))
  ;[0.05098 0.05098 0.05098] Leave Note Reading Mode
  (:`Started`
    (if (`self.BIsPlayerReading`)
      (`self.LeaveNoteHUD`))))

(event `Reload Texture`
  ;[0.05098 0.05098 0.05098] Reload Note Texture
  (bind _outrownames (`DataTableFunctionLibrary.GetDataTableRowNames` "/Game/MyContents/MyTables/DataTables/DT_Notes_MAT.DT_Notes_MAT"))
  (bind _returnvalue (`|GetDataTableRow` "/Game/MyContents/MyTables/DataTables/DT_Notes_MAT.DT_Notes_MAT" (`KismetArrayLibrary.Array_Random` _outrownames))
    (:`then`
      (`PrimitiveComponent.SetMaterial` (`self.PaperSheet_MSH`) 1 (break `/Game/MyContents/MyTables/DataTables/S_NotesMaterials` _returnvalue)))))

(fn `LeaveNoteHUD`
  (`/Engine/EditorBlueprintResources/StandardMacros.DoOnce` false
    (:`Completed`
      ;[1 0.7769 0] Note Sound
      (`self.NoteInteractingSound`)
      (set `self.BIsPlayerReading` false)
      (`SceneComponent.SetVisibility` (`self.PaperSheet_MSH`) true false)
      (`self.EnableInput` (`self.Player Ref`) (`GameplayStatics.GetPlayerController` 0))
      (`Widget.RemoveFromParent` (`self.W_NoteHUD`)))))

(fn `NoteInteractingSound`
  ;[1 0.7769 0] Note Sound
  (`GameplayStatics.PlaySoundAtLocation` "/Game/MyContents/MySounds/PropsSound/PaperSound/Cue/Paper_Interaction_Cue.Paper_Interaction_Cue" (`self.K2_GetActorLocation`) (struct) 1.0 1.0 0.0 null null null null))

(fn `ToggleReading`
  (`/Engine/EditorBlueprintResources/StandardMacros.DoOnce` false
    (:`Completed`
      ;[1 0.7769 0] Note Sound
      (`self.NoteInteractingSound`)
      (`SceneComponent.SetVisibility` (`self.PaperSheet_MSH`) false false)
      (set `self.BIsPlayerReading` true)
      (`self.DisableInput` (`self.Player Ref`) (`GameplayStatics.GetPlayerController` 0))
      (`self.EnableInput` (`GameplayStatics.GetPlayerController` 0))
      ;[0.05098 0.05098 0.05098] Add Text Widget On Screen
      (bind _returnvalue (`|CreateWidget` "/Game/MyContents/MyBlueprints/Widgets/WBP_NotesHUD.WBP_NotesHUD_C"))
      (bind _output_get (set `self.W_NoteHUD` _returnvalue))
      (`UserWidget.AddToViewport` _output_get 0)
      (`Widget.SetVisibility` _output_get "Visible")
      (`/Game/MyContents/MyBlueprints/Widgets/WBP_NotesHUD.Init Widget Note` _output_get (`self.NoteText`)))))

(fn `UserConstructionScript`)