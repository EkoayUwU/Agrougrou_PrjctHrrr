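; BP_Door is a door that toggles open or closed when its Interaction event fires.
; The DoorMovement timeline plays forward or in reverse, lerping the door mesh's world yaw between zero and -90 degrees, regardless of placed orientation.
; A busy flag ignores interactions until the swing finishes, an open flag picks the direction, and debug strings print along the way.
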(event `/Game/MyContents/MyBlueprints/Characters/Player/BPI_Interact.Interaction`
  (if (not (`self.BIsOpening`))
    (set `self.BIsOpening` true)
    (`KismetSystemLibrary.PrintString` "cqczcq")
    (if (not (`self.BIsOpen`))
      (set `self.BIsOpen` true)
      (bind (_direction _lerpvalue) (`Timeline|DoorMovement` :!via `PlayFromStart` :!label _label)
        (:`Update`
          (`SceneComponent.K2_SetWorldRotation` (`self.Door_MSH`) (`KismetMathLibrary.MakeRotator` 0.0 0.0 (`KismetMathLibrary.Lerp` 0.0 -90.0 _lerpvalue)) false false)
          (`KismetSystemLibrary.PrintString` (`KismetStringLibrary.Conv_DoubleToString` _lerpvalue)))
        (:`Finished`
          (set `self.BIsOpening` false)
          (`KismetSystemLibrary.PrintString` "wruff")))
      (else
        (set `self.BIsOpen` false)
        (goto _label :!via `ReverseFromEnd`)))))

(fn `UserConstructionScript`)